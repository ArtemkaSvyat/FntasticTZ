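; Base turtle actor that plays spawn and despawn montages around its movement along the level.
; On BeginPlay it plays the spawn montage, then toggles the Spawn component and calls MoveMe, an empty hook for child Blueprints alongside ExtraMovement.
; The finish event toggles audio, clears stored timers, stops floating pawn movement, plays the despawn montage, then notifies FinishPoint and destroys itself on blend out.
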(event `self.ReceiveBeginPlay`
  ;[1 1 1] Монтаж появления и начало перемещения
  (`|PlayMontage` (`self.SkeletalMesh`) "/Game/TestovoeZadanie/ActorsBPs/Turtle/Spawn_Anim_Montage.Spawn_Anim_Montage"
    (:`OnCompleted`
      (`ActorComponent.ToggleActive` (`self.Spawn`))
      (`self.MoveMe`))))

(event `PlayFinishMontageAndDespawn`
  ;[1 1 1] Финишный монтаж и уничтожение черепах
  (`ActorComponent.ToggleActive` (`self.Audio`))
  (if (`self.CheckForTimerHandles`)
    (for _array_element (`self.Handle`)
      (`KismetSystemLibrary.K2_ClearAndInvalidateTimerHandle` _array_element)))
  (`NavMovementComponent.StopActiveMovement` (`self.FloatingPawnMovement`))
  (`ActorComponent.ToggleActive` (`self.Spawn`))
  (`|PlayMontage` (`self.SkeletalMesh`) "/Game/TestovoeZadanie/ActorsBPs/Turtle/Despawn_Anim_Montage.Despawn_Anim_Montage"
    (:`OnBlendOut`
      (`/Game/TestovoeZadanie/ActorsBPs/FinishPoint.OnTurtleDespawn` (`self.FinishPoint`))
      (`self.K2_DestroyActor`))))

(event `MoveMe`
  ;[1 1 1] Ивенты для чайлдов
)

(event `ExtraMovement`
  ;[1 1 1] Ивенты для чайлдов
)

(fn `CheckForTimerHandles`
  (returns (ReturnValue :type Boolean))
  (return (`KismetSystemLibrary.K2_IsValidTimerHandle` (`|GetArrayItem` (`self.Handle`)))))

(fn `UserConstructionScript`)